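; BP_FLAPPY_MAN is a physics-driven, Flappy Bird-style character that flaps upward when Jump is pressed.
; Each press zeroes the Capsule's linear velocity, then applies an upward force with a one-off AddForce call rather than an impulse.
; Tick adds a downward force only while vertical velocity is positive, damping the rise and leaving the fall free of that extra force.
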(event EventTick
  (params (DeltaSeconds :type Float%20%28single-precision%29))
  (bind _returnvalue (Physics|GetPhysicsLinearVelocity (Variables|Default|GetCapsule) "None"))
  (if (> (.z _returnvalue) 0.0)
    (Physics|AddForce (Variables|Default|GetCapsule) "0.000000,0.000000,-1000.000000" "None" false)))

(event Input|ActionEvents|InputActionJump
  (params (Key :type Key%20Structure :default "None"))
  (:Pressed
    (Physics|SetPhysicsLinearVelocity (Variables|Default|GetCapsule) "0, 0, 0" false "None")
    (Physics|AddForce (Variables|Default|GetCapsule) "0.000000,0.000000,3000.000000" "None" false)))

(fn ConstructionScript)